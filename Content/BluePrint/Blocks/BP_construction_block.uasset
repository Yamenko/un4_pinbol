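; Block grid constructor that lays out child actor blocks and spawns random bonuses through them.
; The construction script adds child actor components on an X by Y padded grid.
; BeginPlay fills the bonus list with new ball, scale and speed, then binds each BP_Destructable's bonus event.
; That event spawns a random bonus at the location of the loop's current ArrayElement, not a passed-in block.
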(event Custom|Spawn%20new%20bonus
  (CallFunction|SpawnBonusFunc (Transformation|GetActorLocation (Variables|/Script/Engine.ChildActorComponent|GetChildActor (stale EventBeginPlay _array_element)))))

(event EventBeginPlay
  (bind _bonuses (Variables|Default|GetBonuses))
  (Utilities|Array|Add _bonuses "/Game/BluePrint/Bonuses/BP_BonusNewBall.BP_BonusNewBall_C")
  (Utilities|Array|Add _bonuses "/Game/BluePrint/Bonuses/BP_BonusScale.BP_BonusScale_C")
  (Utilities|Array|Add _bonuses "/Game/BluePrint/Bonuses/BP_BonusSpeed.BP_BonusSpeed_C")
  (for _array_element (Variables|Default|GetComponentOnScene)
    (bind _asbp_destructable (Utilities|Casting|CastToBP_Destructable (Variables|/Script/Engine.ChildActorComponent|GetChildActor _array_element)))
    (if (Utilities|IsValid _asbp_destructable)
      (EventDispatchers|BindEventtoSpawnBonus _asbp_destructable (delegate Custom|Spawn%20new%20bonus)))))

(fn ConstructionScript
  (for _index (range 0 (Variables|Default|Getx))
    (for _index_2 (range 0 (Variables|Default|Gety))
      (bind _returnvalue (AddComponent|AddChildActorComponent false (Math|Transform|MakeTransform (Math|Vector|MakeVector (Math|Conversions|ToFloat(Integer) (* _index (Variables|Default|Getpadding))) (Math|Conversions|ToFloat(Integer) (* _index_2 (Variables|Default|Getpadding))) 0.0) "0, 0, 0" "1,1,1")))
      (Utilities|Array|Add (Variables|Default|GetComponentOnScene) _returnvalue))))

(fn SpawnBonusFunc
  (params (SpawnLocation :type Vector))
  (Game|SpawnActorfromClass (.OutItem (Utilities|Array|Random (Variables|Default|GetBonuses))) (Math|Transform|MakeTransform SpawnLocation "0, 0, 0" "1,1,1") "Undefined" 0 0))