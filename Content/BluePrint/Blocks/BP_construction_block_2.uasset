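; Block grid Blueprint for a brick-breaker-style game: its construction script lays out static mesh blocks in X by Y loops spaced by Padding.
; A BP_sphere hit swaps a block to SecondMaterial, so the material itself tracks damage.
; A hit on a damaged block spawns a random bonus from Bonuses and destroys that component.
; If it is the last child of the root, QuitGame runs with Background preference.
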(event Collision|EventHit
  (params (MyComp :type Primitive%20Component%20Object%20Reference) (Other :type Actor%20Object%20Reference) (OtherComp :type Primitive%20Component%20Object%20Reference) (bSelfMoved :type Boolean) (HitLocation :type Vector :default "0, 0, 0") (HitNormal :type Vector :default "0, 0, 0") (NormalImpulse :type Vector :default "0, 0, 0") (Hit :type Hit%20Result%20Structure%20%28by%20ref%29))
  (Utilities|Casting|CastToBP_sphere Other)
  (if (== (Variables|Default|GetSecond%20Material) (Rendering|Material|GetMaterial MyComp 0))
    (CallFunction|SpawnBonusFunc HitLocation)
    (bind _finish (CallFunction|CheckFinishGame))
    (if _finish
      (Game|QuitGame 0 "Background" false))
    (Components|DestroyComponent MyComp)
    (else
      (Rendering|Material|SetMaterial MyComp 0 (Variables|Default|GetSecond%20Material)))))

(fn ConstructionScript
  (for _index (range 0 (Variables|Default|Getx))
    (for _index_2 (range 0 (Variables|Default|Gety))
      (AddComponent|AddStaticMeshComponent false (Math|Transform|MakeTransform (Math|Vector|MakeVector (Math|Conversions|ToFloat(Integer) (* _index (Variables|Default|Getpadding))) (Math|Conversions|ToFloat(Integer) (* _index_2 (Variables|Default|Getpadding))) 0.0) "0, 0, 0" "1,1,1")))))

(fn SpawnBonusFunc
  (params (SpawnLocation :type Vector))
  (Game|SpawnActorfromClass (.OutItem (Utilities|Array|Random (Variables|Default|GetBonuses))) (Math|Transform|MakeTransform SpawnLocation "0, 0, 0" "1,1,1") "Undefined" 0 0))

(fn CheckFinishGame
  (return (<= (Class|SceneComponent|GetNumChildrenComponents (Variables|Default|GetDefaultSceneRoot)) 1)))