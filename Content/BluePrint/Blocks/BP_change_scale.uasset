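; BP_change_scale is a block Blueprint whose cube narrows along its X axis based on how many times it has been touched.
; BeginPlay stores the cube's starting scale.
; On actor overlap it runs the parent's handler, then reduces X scale by five percent of the original per CountTouch, leaving Y and Z unchanged.
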(event EventBeginPlay
  (bind _cube (Variables|Default|GetCube))
  (bind _relativescale3d (Variables|/Script/Engine.SceneComponent|GetRelativeScale3D _cube))
  ;[1 1 1] Запоминаем исходный размер
  (Variables|Default|SetStartScale (Math|Vector|MakeVector (.x _relativescale3d) (.y _relativescale3d) (.z _relativescale3d))))

(event Collision|EventActorBeginOverlap
  (params (OtherActor :type Actor%20Object%20Reference))
  (bind _startscale (Variables|Default|GetStartScale))
  (|CallParentFunction OtherActor)
  (if (Utilities|IsValid (Variables|Default|GetCube))
    (Transformation|SetRelativeScale3D (Variables|Default|GetCube) (Math|Vector|MakeVector (* (- 1.0 (* (Variables|Default|Getcount_touch) 0.05)) (.x _startscale)) (.y _startscale) (.z _startscale)))))

(fn ConstructionScript
  (|CallParentFunction))