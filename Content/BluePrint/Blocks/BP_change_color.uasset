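; BP_change_color is a block Blueprint that gives its Cylinder mesh a random color when an actor overlaps it.
; BeginPlay fills a Material array with blue, green and red materials.
; On overlap it runs the parent's handler first, then, if the Cylinder is still valid, applies a randomly picked material to slot 0.
; The pick can repeat the current color.
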(event Collision|EventActorBeginOverlap
  (params (OtherActor :type Actor%20Object%20Reference))
  (bind _material (Variables|Default|GetMaterial))
  (|CallParentFunction OtherActor)
  ;[1 1 1] Проверка что объект еще не уничтожен
  (if (Utilities|IsValid (Variables|Default|GetCylinder))
    ;[1 1 1] Установка нового цвета
    (Rendering|Material|SetMaterial (Variables|Default|GetCylinder) 0 (Utilities|Array|Get(acopy) _material (Math|Random|RandomInteger (Utilities|Array|Length _material))))))

(event EventBeginPlay
  ;[1 1 1] Заполнение массива материалов
  (Variables|Default|SetMaterial (Utilities|Array|MakeArray "/Game/Materials/M_color_blue.M_color_blue" "/Game/Materials/M_color_green.M_color_green" "/Game/Materials/M_color_red.M_color_red")))

(fn ConstructionScript
  (|CallParentFunction))