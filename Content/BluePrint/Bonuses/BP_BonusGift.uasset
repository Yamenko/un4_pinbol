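; BP_BonusGift is a moving bonus pickup sphere for the player slider, with an empty OnNewBonus function, apparently meant for child bonuses to override.
; Tick moves the sphere along its local Y axis by Speed and, through DoOnce, colors it green or red from IsGoodBonus.
; Overlapping BP_player_slide calls OnNewBonus, prints a debug name and destroys the actor, while overlapping a KillZVolume only destroys it.
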(event EventTick
  (params (DeltaSeconds :type Float%20%28single-precision%29))
  (bind _sphere (Variables|Default|GetSphere))
  (Transformation|AddLocalOffset (Variables|Default|GetSphere) (Math|Vector|MakeVector 0.0 (* DeltaSeconds (Variables|Default|GetSpeed)) 0.0) false false)
  ;[1 1 1] перекрашиваем цвет созданного бонуса
  (Utilities|FlowControl|DoOnce false
    (:Completed
      (if (Variables|Default|Getis_goodBonus)
        (Rendering|Material|SetMaterial _sphere 0 "/Game/Materials/M_color_green.M_color_green")
        (else
          (Rendering|Material|SetMaterial _sphere 0 "/Game/Materials/M_color_red.M_color_red"))))))

(event Collision|EventActorBeginOverlap
  (params (OtherActor :type Actor%20Object%20Reference))
  (bind _asbp_player_slide (Utilities|Casting|CastToBP_player_slide OtherActor)
    (:then
      (CallFunction|OnNewBonus _asbp_player_slide)
      (Development|PrintString (Utilities|GetDisplayName (Variables|Default|GetDefaultSceneRoot))))
    (:CastFailed
      (Utilities|Casting|CastToKillZVolume OtherActor)))
  (Actor|DestroyActor))

(fn ConstructionScript)

(fn OnNewBonus
  (params (Slider :type Actor%20Object%20Reference)))