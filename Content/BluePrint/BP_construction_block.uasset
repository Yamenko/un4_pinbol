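; BP_construction_block is an actor that forms a destructible grid of static mesh blocks, broken by BP_sphere hits.
; The construction script adds one mesh component per cell across the X and Y counts, offset by Padding.
; On Hit, a cast filters for BP_sphere and destroys only the struck component, leaving the rest of the grid in place.
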(event EventBeginPlay)

(event Collision|EventActorBeginOverlap
  (params (OtherActor :type Actor%20Object%20Reference)))

(event EventTick
  (params (DeltaSeconds :type Float%20%28single-precision%29)))

(event Collision|EventHit
  (params (MyComp :type Primitive%20Component%20Object%20Reference) (Other :type Actor%20Object%20Reference) (OtherComp :type Primitive%20Component%20Object%20Reference) (bSelfMoved :type Boolean) (HitLocation :type Vector :default "0, 0, 0") (HitNormal :type Vector :default "0, 0, 0") (NormalImpulse :type Vector :default "0, 0, 0") (Hit :type Hit%20Result%20Structure%20%28by%20ref%29))
  (Utilities|Casting|CastToBP_sphere Other)
  (Components|DestroyComponent MyComp))

(fn ConstructionScript
  (bind _padding (Variables|Default|Getpadding))
  (for _index (range 0 (Variables|Default|Getx))
    (for _index_2 (range 0 (Variables|Default|Gety))
      (AddComponent|AddStaticMeshComponent false (Math|Transform|MakeTransform (Math|Vector|MakeVector (Math|Conversions|ToFloat(Integer) (* _index _padding)) (Math|Conversions|ToFloat(Integer) (* _index_2 _padding)) 0.0) "0, 0, 0" "1,1,1")))))